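; Main menu 3D scene actor with a diving bell that becomes the player's view target on BeginPlay.
; Each tick, it deprojects the mouse cursor into the world and rotates its spotlight toward a point 500 units along that ray, so the light follows the cursor.
; MoveBellUp and MoveBellDown nudge the diving bell 100 units vertically with no sweep.
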(event `self.ReceiveBeginPlay`
  (`PlayerController.SetViewTargetWithBlend` (`GameplayStatics.GetPlayerController` 0) self 0.0 "VTBlend_Linear" 0.0 false)
  (`self.SetActorEnableCollision` true))

(event `self.ReceiveTick`
  (params (DeltaSeconds :type "Float (single-precision)"))
  (bind _spotlight (`self.SpotLight`))
  (bind (_worldlocation _worlddirection) (`PlayerController.DeprojectMousePositionToWorld` (`GameplayStatics.GetPlayerController` 0)))
  (`SceneComponent.K2_SetWorldRotation` _spotlight (`KismetMathLibrary.FindLookAtRotation` (`SceneComponent.K2_GetComponentLocation` _spotlight) (+ _worldlocation (* _worlddirection 500.0))) false false))

(fn `MoveBellDown`
  (`SceneComponent.K2_AddRelativeLocation` (`self.DivingBell`) (0.0 0.0 -100.0) false false))

(fn `MoveBellUp`
  (`SceneComponent.K2_AddRelativeLocation` (`self.DivingBell`) (0.0 0.0 100.0) false false))

(fn `UserConstructionScript`)