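; BP_BarkObject plays a timed sequence of bark text lines, triggered once when the player overlaps it.
; The overlap passes the player's InteractionComponent to Bark, which shows the text at the current Index for its paired display duration.
; Bark then increments Index, waits the matching TimeBetweenBarks delay and calls itself again, with no end-of-array check.
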(event `self.OnPlayerOverlapEnter`
  (params (Player :type "SGPlayerCharacter Object Reference") (InteractionComponent :type "SGPlayerInteractionComponent Object Reference"))
  (`/Engine/EditorBlueprintResources/StandardMacros.DoOnce` false
    (:`Completed`
      (`self.Bark` InteractionComponent))))

(event `Bark`
  (params (InteractionComponent :type "SGPlayerInteractionComponent Object Reference"))
  (bind _index (`self.index`))
  (`SGPlayerInteractionComponent.ShowBarkText` InteractionComponent (`|GetArrayItem` (`self.Barks`) _index) (`|GetArrayItem` (`self.DisplayDuration`) _index))
  (bind _output_get (set `self.index` (+ (`self.index`) 1)))
  (`KismetSystemLibrary.Delay` (`|GetArrayItem` (`self.TimeBetweenBarks`) (- _output_get 1)))
  (`self.Bark` InteractionComponent))

(fn `UserConstructionScript`)