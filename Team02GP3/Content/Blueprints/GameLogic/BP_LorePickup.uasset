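; BP_LorePickup is an interactable lore item that adds its data table entry to the player's logbook.
; Player overlap caches the interaction component and logbook and shows a text prompt.
; A successful interaction marks the entry added, shows bark text, plays an update sound, then hides the prompt and disables sphere collision.
; Leaving before pickup joins that same tail, so it also disables the collision.
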(event `self.OnPlayerOverlapEnter`
  (params (Player :type "SGPlayerCharacter Object Reference") (InteractionComponent :type "SGPlayerInteractionComponent Object Reference"))
  (if (not (`self.IsEntryAdded`))
    (set `self.Interaction Component` InteractionComponent)
    (set `self.LogBook` (`SGPlayerInteractionComponent.Logbook` InteractionComponent))
    ;[1 1 1] Show prompt with offset
    (`SGPlayerInteractionComponent.DisplayPromptText` InteractionComponent (`self.TextToShowOnOverlap`) self (`self.TextOffset`) true)))

(event `self.OnInteract`
  (params (Player :type "SGPlayerCharacter Object Reference") (IsKeyPressed :type Boolean))
  (bind (_rowdata_logcategory _rowdata_logname _rowdata_interactiontext) (break `SGLogStruct` (`self.RowData`)))
  (bind (_datahandle_datatable _datahandle_rowname) (break `DataTableRowHandle` (`self.DataHandle`)))
  (bind _returnvalue (`SGLogBook.AddEntry` (`self.LogBook`) _datahandle_rowname true))
  (if _returnvalue
    (set `self.IsEntryAdded` true)
    (`SGPlayerInteractionComponent.ShowBarkText` (`self.Interaction Component`) (`KismetTextLibrary.Conv_TextToString` _rowdata_interactiontext) (`self.BarkDisplayTime`))
    (`GameplayStatics.PlaySound2D` "/Game/Audio/Assets/UI/Logbook_Update.Logbook_Update" 1.0 1.0 0.0 "/Game/Audio/Settings/DefaultSoundConcurrency.DefaultSoundConcurrency" null)
    ;[1 1 1] Hide Prompt
    (`SGPlayerInteractionComponent.DisplayPromptText` (`self.Interaction Component`) "" self (0.0 0.0 100.0) false :!label _label)
    (`PrimitiveComponent.SetCollisionEnabled` (`self.InteractionSphereComponent`) "NoCollision")))

(event `self.OnPlayerOverlapExit`
  (params (Player :type "SGPlayerCharacter Object Reference") (InteractionComponent :type "SGPlayerInteractionComponent Object Reference"))
  ;[1 1 1] Hide Prompt
  (if (not (`self.IsEntryAdded`))
    (goto _label)))

(fn `UserConstructionScript`)