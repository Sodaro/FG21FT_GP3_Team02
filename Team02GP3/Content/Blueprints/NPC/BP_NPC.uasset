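; BP_NPC is an interactable character that shows dialog lines on a text render component.
; On interact, it displays the Content entry at DialogIndex, then advances the index.
; The index wraps to zero at a hardcoded count of two rather than the length of Content, so only the first two lines alternate.
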(event `self.OnInteract`
  (bind _returnvalue (+ (`self.DialogIndex`) 1))
  (`TextRenderComponent.K2_SetText` (`self.TextRender`) (`KismetTextLibrary.Conv_StringToText` (`|GetArrayItem` (`self.Content`) (`self.DialogIndex`))))
  (if (>= _returnvalue 2)
    (set `self.DialogIndex` 0)
    (else
      (set `self.DialogIndex` _returnvalue))))

(fn `UserConstructionScript`)