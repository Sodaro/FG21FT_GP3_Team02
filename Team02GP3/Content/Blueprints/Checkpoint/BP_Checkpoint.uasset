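; One-time checkpoint with a glowing visor, spotlight and audio, which recharges the player's lantern, grants logbook entries and saves the game.
; Player overlap shows or hides a prompt until the checkpoint is used.
; Interaction runs once, switching off glow, light and audio, then staging sounds, log pickup and save with delays.
; Only the last log entry broadcasts its update, after a delay; LightFlicker is an empty stub.
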(event `self.ReceiveBeginPlay`
  (bind _skeletalmesh (`self.SkeletalMesh`))
  (`parent.ReceiveBeginPlay`)
  (`MeshComponent.SetVectorParameterValueOnMaterials` _skeletalmesh "Visor Color" (`KismetMathLibrary.Conv_LinearColorToVector` (`KismetMathLibrary.Conv_ColorToLinearColor` (`self.VisorColor`))))
  (`MeshComponent.SetScalarParameterValueOnMaterials` _skeletalmesh "Emissive intensity" 1.0))

(event `self.OnPlayerOverlapEnter`
  (params (Player :type "SGPlayerCharacter Object Reference") (InteractionComponent :type "SGPlayerInteractionComponent Object Reference"))
  (if (and (`KismetSystemLibrary.IsValid` InteractionComponent) (not (`self.IsUsed`)))
    (bind _output_get (set `self.Interaction Component` InteractionComponent))
    (`SGPlayerInteractionComponent.DisplayPromptText` _output_get (`self.TextToShowOnOverlap`) self (0.0 0.0 100.0) true)))

(event `self.OnInteract`
  (params (Player :type "SGPlayerCharacter Object Reference") (IsKeyPressed :type Boolean))
  (`/Engine/EditorBlueprintResources/StandardMacros.DoOnce` false
    (:`Completed`
      (set `self.IsUsed` true)
      (`SGPlayerCharacterLanternComponent.ChargeLantern` (`SGPlayerCharacter.PlayerLantern` Player))
      (`GameplayStatics.PlaySound2D` "/Game/Audio/Assets/Gameplay/Body_Loot_General.Body_Loot_General" 1.0 1.0 0.0 "/Game/Audio/Settings/DefaultSoundConcurrency.DefaultSoundConcurrency" null false)
      (`self.DisableCheckpointLightAndAudio`)
      (`KismetSystemLibrary.Delay` 1.0)
      (`GameplayStatics.PlaySound2D` "/Game/Audio/Assets/Gameplay/Light_Restore-2.Light_Restore-2" 1.0 1.0 0.0 "/Game/Audio/Settings/DefaultSoundConcurrency.DefaultSoundConcurrency" null false)
      (`self.PickUpLogEntries` (`SGPlayerCharacter.InteractionComponent` Player))
      (`KismetSystemLibrary.Delay` 0.2)
      (`SGPlayerCharacter.SaveGame` Player))))

(event `self.OnPlayerOverlapExit`
  (params (Player :type "SGPlayerCharacter Object Reference") (InteractionComponent :type "SGPlayerInteractionComponent Object Reference"))
  ;[1 1 1] Hide Prompt
  (`SGPlayerInteractionComponent.DisplayPromptText` (`self.Interaction Component`) "" self (0.0 0.0 100.0) false))

(event `LightFlicker`)

(event `DisableCheckpointLightAndAudio`
  (bind _interaction_component (`self.Interaction Component`))
  (`MeshComponent.SetScalarParameterValueOnMaterials` (`self.SkeletalMesh`) "Emissive intensity" 0.0)
  (`SceneComponent.SetVisibility` (`self.Spotlight`) false false)
  (`AudioComponent.Stop` (`self.Audio`))
  (`/Engine/EditorBlueprintResources/StandardMacros.IsValid` _interaction_component
    (:`Is Valid`
      (`SGPlayerInteractionComponent.DisplayPromptText` _interaction_component "" self (0.0 0.0 100.0) false))))

(event `PickUpLogEntries`
  (params (InteractionComponent :type "SGPlayerInteractionComponent Object Reference"))
  (bind _logbook (`SGPlayerInteractionComponent.Logbook` InteractionComponent))
  (for (_array_element _array_index) (`self.EntriesToAdd`)
    (if (== _array_index (- (`KismetArrayLibrary.Array_Length` (`self.EntriesToAdd`)) 1))
      (`KismetSystemLibrary.Delay` 2.0)
      (`SGLogBook.AddEntry` _logbook (`.RowName` (break `DataTableRowHandle` _array_element)) true)
      (`GameplayStatics.PlaySound2D` "/Game/Audio/Assets/UI/Logbook_Update.Logbook_Update" 1.0 1.0 0.0 "/Game/Audio/Settings/DefaultSoundConcurrency.DefaultSoundConcurrency" null false)
      (else
        (`SGLogBook.AddEntry` _logbook (`.RowName` (break `DataTableRowHandle` _array_element)) false)))))

(fn `UserConstructionScript`)