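; Player pawn that handles pause input and a UV flashlight that flags enemies caught in it.
; Escape and P share a FlipFlop that creates the pause menu and pauses, then removes it and resumes.
; UVLight overlaps set or clear the SeenByFlashlight Blackboard key on each EnemyCharacter.
; Right mouse toggles IsHoldingLight and prints the state, but the overlap logic does not check that flag.
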(event `Key|Escape` :paused true
  (params (Key :type "Key Structure"))
  (:`Pressed`
    (`/Engine/EditorBlueprintResources/StandardMacros.FlipFlop` :!label _label
      (:`A`
        (bind _returnvalue (`|CreateWidget` "/Game/Blueprints/UI/PauseMenu/WBP_PauseMenu.WBP_PauseMenu_C"))
        (`UserWidget.AddToViewport` _returnvalue 0)
        (`GameplayStatics.SetGamePaused` true))
      (:`B`
        (`Widget.RemoveFromParent` _returnvalue)
        (`GameplayStatics.SetGamePaused` false)))))

(event `Key|P` :paused true
  (params (Key :type "Key Structure"))
  (:`Pressed`
    (goto _label)))

(event `self.UVLight.OnComponentBeginOverlap`
  (params (OverlappedComponent :type "PrimitiveComponent Object Reference") (OtherActor :type "Actor Object Reference") (OtherComp :type "PrimitiveComponent Object Reference") (OtherBodyIndex :type Integer) (bFromSweep :type Boolean) (SweepResult :type "HitResult Structure (by ref)"))
  (bind _asenemy_character (cast `/Game/AITest/EnemyCharacter` OtherActor))
  (`BlackboardComponent.SetValueAsBool` (`AIBlueprintHelperLibrary.GetBlackboard` _asenemy_character) "SeenByFlashlight" true))

(event `self.UVLight.OnComponentEndOverlap`
  (params (OverlappedComponent :type "PrimitiveComponent Object Reference") (OtherActor :type "Actor Object Reference") (OtherComp :type "PrimitiveComponent Object Reference") (OtherBodyIndex :type Integer))
  (bind _asenemy_character (cast `/Game/AITest/EnemyCharacter` OtherActor))
  (`BlackboardComponent.SetValueAsBool` (`AIBlueprintHelperLibrary.GetBlackboard` _asenemy_character) "SeenByFlashlight" false))

(event `Key|RightMouseButton`
  (params (Key :type "Key Structure"))
  (:`Pressed`
    (if (`self.IsHoldingLight`)
      (set `self.IsHoldingLight` false)
      (`KismetSystemLibrary.PrintString` "lights off")
      (else
        (set `self.IsHoldingLight` true)
        (`KismetSystemLibrary.PrintString` "lights on")))))

(fn `UserConstructionScript`)