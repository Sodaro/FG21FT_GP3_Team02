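; Player character Blueprint with a UV-capable lantern, interaction, pause menu, looping breath-and-bubble effects and debug teleport keys.
; Capsule overlaps collect interactables, or let EnemyTriggers configure and teleport the single EnemyCharacter and start its blackboard-driven behavior.
; UV light overlaps flag the enemy as seen, while lantern events recolor the visor and toggle emissive glow.
; Death fades out, resets the enemy and last trigger, then loads the saved game.
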(event `self.ReceiveBeginPlay`
  (`MeshComponent.SetScalarParameterValueOnMaterials` (`self.Mesh`) "Emissive intensity" 1.0)
  (`self.PlayBreathSound`)
  (if (`self.DeleteSaveDataOnStart`)
    (`GameplayStatics.DeleteGameInSlot` "SaveSlot")))

(event `self.ReceiveTick`
  (params (DeltaSeconds :type "Float (single-precision)")))

(event `Key|Escape` :paused true
  (params (Key :type "Key Structure"))
  ;[1 1 1] Pause Menu
  (:`Pressed`
    (`/Engine/EditorBlueprintResources/StandardMacros.FlipFlop` :!label _label
      (:`A`
        (bind _returnvalue (`|CreateWidget` "/Game/Blueprints/UI/PauseMenu/WBP_PauseMenu.WBP_PauseMenu_C"))
        (bind _output_get (set `self.PauseMenu` _returnvalue))
        (`UserWidget.AddToViewport` _output_get 0)
        (`GameplayStatics.SetGamePaused` true))
      (:`B`
        (`Widget.RemoveFromParent` (`self.PauseMenu`))
        (`GameplayStatics.SetGamePaused` false)))))

(event `Key|P` :paused true
  (params (Key :type "Key Structure"))
  ;[1 1 1] Pause Menu
  (:`Pressed`
    (goto _label)))

(event `self.CapsuleComponent.OnComponentBeginOverlap`
  (params (OverlappedComponent :type "PrimitiveComponent Object Reference") (OtherActor :type "Actor Object Reference") (OtherComp :type "PrimitiveComponent Object Reference") (OtherBodyIndex :type Integer) (bFromSweep :type Boolean) (SweepResult :type "HitResult Structure (by ref)"))
  ;[1 1 1] TODO: Move this to C++
  (bind _assginteractable_actor (cast `SGInteractableActor` OtherActor)
    (:`then`
      (`BlueprintSetLibrary.Set_Add` (`self.InteractableObjects`) _assginteractable_actor))
    (:`CastFailed`
      ;[1 1 1] EnemyTrigger
      (bind _asenemy_trigger (cast `/Game/AITest/EnemyTrigger` OtherActor))
      (set `self.LastEnemyTrigger` _asenemy_trigger)
      (if (not (`/Game/AITest/EnemyTrigger.IsTriggered` _asenemy_trigger))
        (bind _returnvalue (`GameplayStatics.GetActorOfClass` "/Game/AITest/EnemyCharacter.EnemyCharacter_C"))
        (bind _output_get (set `/Game/AITest/EnemyCharacter.SpawnLocation` (`/Game/AITest/EnemyTrigger.SpawnLocation` _asenemy_trigger) _returnvalue))
        (set `/Game/AITest/EnemyCharacter.RunawayLocation` (`/Game/AITest/EnemyTrigger.RunawayLocation` _asenemy_trigger) _returnvalue)
        (set `/Game/AITest/EnemyCharacter.Lifes` (`/Game/AITest/EnemyTrigger.Lifes` _asenemy_trigger) _returnvalue)
        (set `/Game/AITest/EnemyCharacter.TempLife` (`/Game/AITest/EnemyCharacter.Lifes` _returnvalue) _returnvalue)
        (set `/Game/AITest/EnemyCharacter.ChasingSpeed` (`/Game/AITest/EnemyTrigger.ChasingSpeed` _asenemy_trigger) _returnvalue)
        (set `/Game/AITest/EnemyCharacter.AttackRange` (`/Game/AITest/EnemyTrigger.AttackRange` _asenemy_trigger) _returnvalue)
        (`self.K2_TeleportTo` _returnvalue _output_get (`KismetMathLibrary.FindLookAtRotation` (`self.K2_GetActorLocation` _returnvalue) (`self.K2_GetActorLocation` self)))
        (set `/Game/AITest/EnemyTrigger.IsTriggered` true _asenemy_trigger)
        (if (`/Game/AITest/EnemyTrigger.SpawnAndJustMoveToRunawayLocation` _asenemy_trigger)
          (bind _returnvalue_2 (`AIBlueprintHelperLibrary.GetBlackboard` _returnvalue))
          (`BlackboardComponent.SetValueAsBool` _returnvalue_2 "SpawnAndJustMoveToRunawayLocation" true)
          (else
            (`BlackboardComponent.SetValueAsBool` _returnvalue_2 "StartBehavior" true)))))))

(event `self.CapsuleComponent.OnComponentEndOverlap`
  (params (OverlappedComponent :type "PrimitiveComponent Object Reference") (OtherActor :type "Actor Object Reference") (OtherComp :type "PrimitiveComponent Object Reference") (OtherBodyIndex :type Integer))
  ;[1 1 1] TODO: Move this to C++
  (bind _assginteractable_actor (cast `SGInteractableActor` OtherActor))
  (`BlueprintSetLibrary.Set_Remove` (`self.InteractableObjects`) _assginteractable_actor))

(event `InputAction|Interact` :overrideparent false
  (params (Key :type "Key Structure"))
  ;[1 1 1] TODO: Move this to C++
  (:`Pressed`
    (bind _result (`BlueprintSetLibrary.Set_ToArray` (`self.InteractableObjects`)))
    (for _array_element _result
      (if (`KismetSystemLibrary.IsValid` _array_element)
        (`SGInteractableActor.OnInteract` _array_element self false)))))

(event `self.PlayerLantern.LanternEnabledChanged`
  (params (Value :type Boolean))
  ;[1 1 1] Set light on
  (bind _output_get (set `self.IsHoldingLight` Value))
  (`MeshComponent.SetScalarParameterValueOnMaterials` (`self.Mesh`) "Emissive intensity" (select `bool` _output_get :`true` 1.0 :!type "Float (single-precision)")))

(event `Death`
  ;[1 1 1] Death
  (`self.DisableInput` null)
  (bind _returnvalue (`|CreateWidget` "/Game/AITest/Fade_Out.Fade_Out_C"))
  (`UserWidget.AddToViewport` _returnvalue 0)
  (`KismetSystemLibrary.Delay` 3.0)
  (bind _returnvalue_2 (`GameplayStatics.GetActorOfClass` "/Game/AITest/EnemyCharacter.EnemyCharacter_C"))
  (`self.K2_TeleportTo` :`self` _returnvalue_2 :`DestLocation` (`/Game/AITest/EnemyCharacter.SpawnLocation` _returnvalue_2))
  (bind _asenemy_trigger (cast `/Game/AITest/EnemyTrigger` (`self.LastEnemyTrigger`)))
  (set `/Game/AITest/EnemyTrigger.IsTriggered` false _asenemy_trigger)
  (`self.LoadGame`)
  (bind _returnvalue_3 (`|CreateWidget` "/Game/AITest/Fade_In.Fade_In_C"))
  (`UserWidget.AddToViewport` _returnvalue_3 0)
  (`self.EnableInput` null))

(event `self.UV-Light.OnComponentBeginOverlap`
  (params (OverlappedComponent :type "PrimitiveComponent Object Reference") (OtherActor :type "Actor Object Reference") (OtherComp :type "PrimitiveComponent Object Reference") (OtherBodyIndex :type Integer) (bFromSweep :type Boolean) (SweepResult :type "HitResult Structure (by ref)"))
  ;[1 0.1543 0.1244] Enemy Light Reaction
  (bind _asenemy_character (cast `/Game/AITest/EnemyCharacter` OtherActor))
  (`BlackboardComponent.SetValueAsBool` (`AIBlueprintHelperLibrary.GetBlackboard` _asenemy_character) "SeenByFlashlight" true)
  (set `/Game/AITest/EnemyCharacter.SeenByFlashLight` true _asenemy_character))

(event `self.UV-Light.OnComponentEndOverlap`
  (params (OverlappedComponent :type "PrimitiveComponent Object Reference") (OtherActor :type "Actor Object Reference") (OtherComp :type "PrimitiveComponent Object Reference") (OtherBodyIndex :type Integer))
  ;[1 0.1543 0.1244] Enemy Light Reaction
  (bind _asenemy_character (cast `/Game/AITest/EnemyCharacter` OtherActor))
  (`BlackboardComponent.SetValueAsBool` (`AIBlueprintHelperLibrary.GetBlackboard` _asenemy_character) "SeenByFlashlight" false)
  (set `/Game/AITest/EnemyCharacter.SeenByFlashLight` false _asenemy_character)
  (set `/Game/AITest/EnemyCharacter.TempLightTolerantTime` 0.0 _asenemy_character))

(event `self.PlayerLantern.UVEnabledChanged`
  (params (Value :type Boolean))
  (bind _playerlantern (`self.PlayerLantern`))
  ;[1 1 1] Visor Colors
  (`MeshComponent.SetVectorParameterValueOnMaterials` (`self.Mesh`) "Visor Color" (select `bool` Value :`false` (`KismetMathLibrary.Conv_LinearColorToVector` (`KismetMathLibrary.Conv_ColorToLinearColor` (`SGPlayerCharacterLanternComponent.NormalColor` _playerlantern))) :`true` (`KismetMathLibrary.Conv_LinearColorToVector` (`KismetMathLibrary.Conv_ColorToLinearColor` (`SGPlayerCharacterLanternComponent.UVColor` _playerlantern))))))

(event `Key|One`
  (params (Key :type "Key Structure"))
  (:`Pressed`
    (set `self.i` 0)
    (if (not (`KismetSystemLibrary.IsPackagedForDistribution`)) :!label _label_2
      (`self.Teleport` (`self.i`)))))

(event `Key|Two`
  (params (Key :type "Key Structure"))
  (:`Pressed`
    (set `self.i` 1)
    (goto _label_2)))

(event `Key|Three`
  (params (Key :type "Key Structure"))
  (:`Pressed`
    (set `self.i` 2)
    (goto _label_2)))

(event `Key|Four`
  (params (Key :type "Key Structure"))
  (:`Pressed`
    (set `self.i` 3)
    (goto _label_2)))

(event `PlayBreathSound`
  (bind _breathingaudiocomponent (`self.BreathingAudioComponent`))
  ;[0.2474 1 0] Breathing Sounds
  (`KismetSystemLibrary.Delay` (`KismetMathLibrary.RandomFloatInRange` (`self.MinDelayBetweenBreaths`) (`self.MaxDelayBetweenBreaths`)))
  (if (== (`KismetMathLibrary.RandomInteger` 2) 0)
    (`AudioComponent.SetSound` _breathingaudiocomponent "/Game/Audio/Assets/Player/Player_Breathe-var1.Player_Breathe-var1")
    (else
      (`AudioComponent.SetSound` _breathingaudiocomponent "/Game/Audio/Assets/Player/Player_Breathe-var2.Player_Breathe-var2")))
  (`AudioComponent.Play` _breathingaudiocomponent 0.0)
  (`self.DoBubbleBurst` (`SoundBase.Duration` (`AudioComponent.Sound` _breathingaudiocomponent)))
  (`self.PlayBreathSound`))

(event `Key|Five`
  (params (Key :type "Key Structure"))
  (:`Pressed`
    (set `self.i` 4)
    (goto _label_2)))

(event `Key|Six`
  (params (Key :type "Key Structure"))
  (:`Pressed`
    (set `self.i` 5)
    (goto _label_2)))

(event `Key|Seven`
  (params (Key :type "Key Structure"))
  (:`Pressed`
    (set `self.i` 6)
    (goto _label_2)))

(event `DoBubbleBurst`
  (params (Duration :type "Float (double-precision)"))
  (bind _niagarabubbles (`self.NiagaraBubbles`))
  (`ActorComponent.Activate` _niagarabubbles false)
  (`KismetSystemLibrary.Delay` Duration)
  (`ActorComponent.Deactivate` _niagarabubbles))

(fn `UserConstructionScript`)