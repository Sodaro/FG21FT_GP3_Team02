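; Dialogue actor for talkable NPCs that shows a talk prompt on overlap and aborts the conversation when the player leaves.
; Interacting lazily creates a WBP_Dialogue widget, advances active dialogue, or plays an index from its ConversationsDataTable row selected by ConversationIndex.
; A completion counter steps through primary, secondary and third dialogues, then cycles between two blurbs.
; Unset (-1) entries are skipped until the counter wraps.
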(event `self.OnPlayerOverlapExit`
  (params (Player :type "SGPlayerCharacter Object Reference") (InteractionComponent :type "SGPlayerInteractionComponent Object Reference"))
  (bind _dialoguewidget (`self.DialogueWidget`))
  ;[1 1 1] Quit dialogue when the player moves away from the NPC
  (`SGPlayerInteractionComponent.DisplayPromptText` InteractionComponent "" self (0.0 0.0 0.0) false)
  ;;[1 1 1] Has the dialogue widget been initialized?
  (if (`KismetSystemLibrary.IsValid` _dialoguewidget)
    (`/Game/Blueprints/Dialogue/WBP_Dialogue.AbortDialogue` _dialoguewidget)))

(event `self.OnPlayerOverlapEnter`
  (params (Player :type "SGPlayerCharacter Object Reference") (InteractionComponent :type "SGPlayerInteractionComponent Object Reference"))
  ;[1 1 1] Quit dialogue when the player moves away from the NPC
  (`SGPlayerInteractionComponent.DisplayPromptText` InteractionComponent "[E] Talk" self (0.0 0.0 100.0) true))

(event `On Dialogue Complete`
  ;[1 1 1] When the dialogue is done, change what dialogue to play
  (bind _result (`/Engine/EditorBlueprintResources/StandardMacros.IncrementInt` (`self.DialoguesCompleted`))
    (:`  `
      (if (> _result 4)
        (set `self.DialoguesCompleted` 3)))))

(event `self.OnInteract`
  (params (Player :type "SGPlayerCharacter Object Reference") (IsKeyPressed :type Boolean))
  ;[1 1 1] Has the dialogue widget been initialized?
  (if (`KismetSystemLibrary.IsValid` (`self.DialogueWidget`))
    ;[1 1 1] Check if the dialogue widget is busy doing something
    (if (`/Game/Blueprints/Dialogue/WBP_Dialogue.isActive` (`self.DialogueWidget`))
      (`/Game/Blueprints/Dialogue/WBP_Dialogue.interactDuringDialogue` (`self.DialogueWidget`))
      (else
        ;[1 1 1] Play the relevant dialogue
        (bind _outrownames (`DataTableFunctionLibrary.GetDataTableRowNames` "/Game/Blueprints/Dialogue/ConversationsDataTable.ConversationsDataTable" :!label _label))
        (bind _returnvalue (`|GetDataTableRow` "/Game/Blueprints/Dialogue/ConversationsDataTable.ConversationsDataTable" (`|GetArrayItem` _outrownames (`self.ConversationIndex`)))
          (:`then`
            (bind (_primarydialogueindex _secondarydialogueindex _thirddialogueindex _blurb1 _blurb2) (break `/Game/Blueprints/Dialogue/NPCConversationStruct` _returnvalue))
            (bind _returnvalue_2 (select `int` (`self.DialoguesCompleted`) :`0` _primarydialogueindex :`1` _secondarydialogueindex :`2` _thirddialogueindex :`3` _blurb1 :`4` _blurb2))
            (if (== _returnvalue_2 -1) :!label _label_2
              (bind _result (`/Engine/EditorBlueprintResources/StandardMacros.IncrementInt` (`self.DialoguesCompleted`))
                (:`  `
                  (if (> _result 4)
                    (set `self.DialoguesCompleted` 3)
                    (else
                      (goto _label_2)))))
              (else
                (`/Game/Blueprints/Dialogue/WBP_Dialogue.playText` (`self.DialogueWidget`) _returnvalue_2 self)))))))
    (else
      ;[1 1 1] Initialize dialogue widget
      (bind _returnvalue_3 (`|CreateWidget` "/Game/Blueprints/Dialogue/WBP_Dialogue.WBP_Dialogue_C" (`GameplayStatics.GetPlayerController` 0)))
      (bind _output_get (set `self.DialogueWidget` _returnvalue_3))
      (`UserWidget.AddToViewport` _output_get 0)
      (goto _label))))

(fn `UserConstructionScript`)